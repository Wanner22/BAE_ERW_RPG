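; BP_CameraChanger is a trigger that toggles the view between the player's camera and a TargetCamera.
; Each BP_TopDownCharacter overlap of its Box alternates through a FlipFlop, asking the top-down controller to switch cameras.
; While TargetCamera is active (IsPlayerCam true, despite the name), Tick slides it along Y with the pawn, offset by CamYOffset.
; Switching back returns it to the start position cached at BeginPlay.
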(event OnComponentBeginOverlap(Box)
  (params (OverlappedComponent :type Primitive%20Component%20Object%20Reference) (OtherActor :type Actor%20Object%20Reference) (OtherComp :type Primitive%20Component%20Object%20Reference) (OtherBodyIndex :type Integer) (bFromSweep :type Boolean) (SweepResult :type Hit%20Result%20Structure%20%28by%20ref%29))
  (Utilities|Casting|CastToBP_TopDownCharacter OtherActor)
  (Utilities|FlowControl|FlipFlop
    (:A
      (Default|ChangeCamera (CallFunction|GetTopDownController) (Variables|Default|GetTargetCamera))
      (Variables|Default|SetIsPlayerCam true))
    (:B
      (Default|CameratoPlayer (CallFunction|GetTopDownController))
      (Transformation|SetActorLocation (Variables|Default|GetTargetCamera) (Variables|Default|GetStartPos) false false)
      (Variables|Default|SetIsPlayerCam false))))

(event EventBeginPlay
  (Variables|Default|SetStartPos (Transformation|GetActorLocation (Variables|Default|GetTargetCamera))))

(event EventTick
  (params (DeltaSeconds :type Float%20%28single-precision%29))
  (bind _startpos (Variables|Default|GetStartPos))
  (if (Variables|Default|GetIsPlayerCam)
    (Transformation|SetActorLocation (Variables|Default|GetTargetCamera) (Math|Vector|MakeVector (.x _startpos) (- (.y (Transformation|GetActorLocation (Game|Player|GetPlayerPawn 0))) (Variables|Default|GetCamYOffset)) (.z _startpos)) false false)))

(fn ConstructionScript)