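; Base interactable actor that registers itself with the top-down controller's Interractables array while another actor overlaps it.
; Begin overlap adds it uniquely and shows InteractText if it is the last array entry; end overlap removes it and hides the text.
; The text starts hidden, and while it is visible Tick rotates it to face the BP_TopDownCharacter camera.
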(event EventBeginPlay
  (Rendering|SetVisibility (Variables|Default|GetInteractText) false false))

(event Collision|EventActorBeginOverlap
  (params (OtherActor :type Actor%20Object%20Reference))
  (bind _playercontroller (CallFunction|GetTopDownController))
  (bind _self self)
  (bind _interractables (Variables|/Game/TopDown/Blueprints/BP_TopDownController.BP_TopDownController_C|GetInterractables _playercontroller))
  (CallFunction|AddInterractable _self)
  (if (== (Utilities|Array|FindItem _interractables _self) (Utilities|Array|LastIndex _interractables))
    (Rendering|SetVisibility (Variables|Default|GetInteractText) true false)))

(event EventTick
  (params (DeltaSeconds :type Float%20%28single-precision%29))
  (Utilities|FlowControl|Sequence
    (:then_0
      ;[0.15 0.15 0.15 0.5] Text is facing the camera when visible
      (if (Rendering|IsVisible (Variables|Default|GetInteractText))
        (bind _asbp_top_down_character (Utilities|Casting|CastToBP_TopDownCharacter (Game|Player|GetPlayerPawn 0)))
        (Transformation|SetWorldRotation (Variables|Default|GetInteractText) (Math|Rotator|FindLookatRotation (Transformation|GetWorldLocation (Variables|Default|GetInteractText)) (Transformation|GetWorldLocation (Variables|/Game/TopDown/Blueprints/BP_TopDownCharacter.BP_TopDownCharacter_C|GetCamera _asbp_top_down_character))) false false)))))

(event Collision|EventActorEndOverlap
  (params (OtherActor :type Actor%20Object%20Reference))
  (bind _self self)
  (CallFunction|RemoveInterractable _self _self)
  (Rendering|SetVisibility (Variables|Default|GetInteractText) false false))

(fn ConstructionScript)

(fn AddInterractable
  (params (Interractable :type BP%20Interractable%20Object%20Reference%20%28by%20ref%29))
  (bind _returnvalue (Utilities|Array|AddUnique (Variables|/Game/TopDown/Blueprints/BP_TopDownController.BP_TopDownController_C|GetInterractables (CallFunction|GetTopDownController)) Interractable))
  (return _returnvalue))

(fn RemoveInterractable
  (params (Interractable :type BP%20Interractable%20Object%20Reference%20%28by%20ref%29))
  (Utilities|Array|RemoveItem (Variables|/Game/TopDown/Blueprints/BP_TopDownController.BP_TopDownController_C|GetInterractables (CallFunction|GetTopDownController)) Interractable))