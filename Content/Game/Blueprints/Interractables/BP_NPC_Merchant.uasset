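; Interactable merchant NPC that shows an "E to shop" prompt and opens a shop UI when used.
; BeginPlay creates the shop widget with a back-reference to the merchant; Interact switches the top-down controller's camera to it and opens the shop after the blend delay.
; StartShop rebuilds one slot widget per ItemsToSell entry and refreshes the money display.
; ExitShop removes the widget and returns the camera to the player.
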(event EventBeginPlay
  (CallFunction|SetInteractText "E to shop")
  (bind _returnvalue (UserInterface|CreateWidget "/Game/Game/UI/Shop/WBP_Shop.WBP_Shop_C"))
  (bind _output_get (Variables|Default|SetShopWidget _returnvalue))
  (Variables|/Game/Game/UI/Shop/WBP_Shop.WBP_Shop_C|SetMerchant _output_get self))

(event Collision|EventActorBeginOverlap
  (params (OtherActor :type Actor%20Object%20Reference))
  (|CallParentFunction OtherActor) ; This node is disabled and will not be called.\nDrag off pins to build functionality.
)

(event EventTick
  (params (DeltaSeconds :type Float%20%28single-precision%29))
  (|CallParentFunction DeltaSeconds) ; This node is disabled and will not be called.\nDrag off pins to build functionality.
)

(event EventInteract
  (Default|ChangeCamera (CallFunction|GetTopDownController) self)
  (Utilities|FlowControl|Delay (+ (Variables|Default|GetCamBlendTime) 0.4))
  (CallFunction|StartShop))

(fn ConstructionScript
  (|CallParentFunction))

(fn ExitShop
  (Widget|RemovefromParent (Variables|Default|GetShopWidget))
  (Default|CameratoPlayer (CallFunction|GetTopDownController)))

(fn StartShop
  (bind _shopwidget (Variables|Default|GetShopWidget))
  (UserInterface|Viewport|AddtoViewport _shopwidget 0)
  (Widget|Panel|ClearChildren (Variables|/Game/Game/UI/Shop/WBP_Shop.WBP_Shop_C|GetHorizontalBox_0 _shopwidget))
  (for _array_element (Variables|Default|GetItemsToSell)
    ;[0.15 0.15 0.15 0.5] Sets every item in the item shop
    (bind _returnvalue (UserInterface|CreateWidget "/Game/Game/UI/Shop/WBP_ShopSlot.WBP_ShopSlot_C"))
    (bind _output_get (Variables|Default|SetShopSlotWidget _returnvalue))
    (Appearance|SetBrushfromTexture (Variables|/Game/Game/UI/Shop/WBP_ShopSlot.WBP_ShopSlot_C|GetItemImage _output_get) (Variables|/Game/Game/Blueprints/Datas/BP_DA_Item.BP_DA_Item_C|GetIcon _array_element) false)
    (Variables|/Script/UMG.TextBlock|SetText (Variables|/Game/Game/UI/Shop/WBP_ShopSlot.WBP_ShopSlot_C|GetPriceText (Variables|Default|GetShopSlotWidget)) (Utilities|Text|ToText(String) (Utilities|String|Append (Utilities|String|ToString(Integer) (Variables|/Game/Game/Blueprints/Datas/BP_DA_Item.BP_DA_Item_C|GetPrice _array_element)) "$")))
    (Variables|/Script/UMG.TextBlock|SetText (Variables|/Game/Game/UI/Shop/WBP_ShopSlot.WBP_ShopSlot_C|GetItemName (Variables|Default|GetShopSlotWidget)) (Variables|/Game/Game/Blueprints/Datas/BP_DA_Item.BP_DA_Item_C|GetName _array_element))
    (Variables|/Game/Game/UI/Shop/WBP_ShopSlot.WBP_ShopSlot_C|SetItem (Variables|Default|GetShopSlotWidget) _array_element)
    (Default|UpdateMoney (CallFunction|GetTopDownController))
    (Class|HorizontalBox|AddChildtoHorizontalBox (Variables|/Game/Game/UI/Shop/WBP_Shop.WBP_Shop_C|GetHorizontalBox_0 (Variables|Default|GetShopWidget)) (Variables|Default|GetShopSlotWidget))))