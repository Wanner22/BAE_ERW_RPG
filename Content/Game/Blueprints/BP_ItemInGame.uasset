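; BP_ItemInGame is a world pickup actor that adds its assigned Item to the player's inventory.
; Its construction script applies the Item's mesh to the static mesh component when the Item is valid.
; When a BP_TopDownCharacter overlaps the sphere, it adds the Item through the top-down controller, refreshes the inventory slots and destroys itself.
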(event OnComponentBeginOverlap(Sphere)
  (params (OverlappedComponent :type Primitive%20Component%20Object%20Reference) (OtherActor :type Actor%20Object%20Reference) (OtherComp :type Primitive%20Component%20Object%20Reference) (OtherBodyIndex :type Integer) (bFromSweep :type Boolean) (SweepResult :type Hit%20Result%20Structure%20%28by%20ref%29))
  (Utilities|Casting|CastToBP_TopDownCharacter OtherActor)
  (Default|AddItem (CallFunction|GetTopDownController) (Variables|Default|GetItem))
  (Default|UpdateInventorySlots (CallFunction|GetTopDownController))
  (Actor|DestroyActor))

(event EventBeginPlay)

(event EventTick
  (params (DeltaSeconds :type Float%20%28single-precision%29)))

(fn ConstructionScript
  (bind _item (Variables|Default|GetItem)
    (:then
      (Components|StaticMesh|SetStaticMesh (Variables|Default|GetStaticMesh) (Variables|/Game/Game/Blueprints/Datas/BP_DA_Item.BP_DA_Item_C|GetMesh _item)))
    (:else)))