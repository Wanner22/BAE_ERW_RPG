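; BP_Fireball is a launchable spell projectile that damages the top-down player or enemies on contact.
; LaunchSpell applies an impulse to its sphere along the caster pawn's forward vector, scaled by LaunchSpeed.
; On overlap it skips the caster, sends damage to the player or enemy AI controller, then destroys itself, with temporary invincibility for the player.
; An unused fireball destroys itself after a short delay.
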(event OnComponentBeginOverlap(SphereCollision)
  (params (OverlappedComponent :type Primitive%20Component%20Object%20Reference) (OtherActor :type Actor%20Object%20Reference) (OtherComp :type Primitive%20Component%20Object%20Reference) (OtherBodyIndex :type Integer) (bFromSweep :type Boolean) (SweepResult :type Hit%20Result%20Structure%20%28by%20ref%29))
  (bind _playercontroller (CallFunction|GetTopDownController))
  (Utilities|Casting|CastToBP_TopDownCharacter OtherActor
    (:then
      (if (!= (Variables|Default|GetCurrentUser) _playercontroller)
        (Default|TakeDamages _playercontroller 1e+01 1.0)
        (Actor|DestroyActor)))
    (:CastFailed
      (bind _asbp_top_down_enemy_character (Utilities|Casting|CastToBP_TopDownEnemy_Character OtherActor))
      (bind _asbp_enemy_ai_controller (Utilities|Casting|CastToBP_EnemyAI_Controller (Pawn|GetController _asbp_top_down_enemy_character)))
      (if (!= _asbp_enemy_ai_controller (Variables|Default|GetCurrentUser))
        (Default|TakeDamages _asbp_enemy_ai_controller 1e+01)
        (Actor|DestroyActor)))))

(event EventBeginPlay
  (Utilities|FlowControl|Delay 3.0)
  (Actor|DestroyActor))

(fn ConstructionScript)

(fn LaunchSpell
  (Physics|AddImpulse (Variables|Default|GetSphere) (* (Variables|Default|GetLaunchSpeed) (Transformation|GetActorForwardVector (Pawn|GetControlledPawn (Variables|Default|GetCurrentUser)))) "None" false))