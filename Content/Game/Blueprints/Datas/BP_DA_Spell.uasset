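; BP_DA_Spell is a spell data asset whose Use function casts a spell for either the player or an enemy AI.
; It casts the user to BP_TopDownController, falling back to BP_EnemyAI_Controller, and has that controller spawn ActorClass as a non-zone spell.
; The spawned actor records the controller as CurrentUser, then LaunchSpell fires and Use returns true.
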(fn Use
  (params (User :type Controller%20Object%20Reference))
  (bind _asbp_top_down_controller (Utilities|Casting|CastToBP_TopDownController User)
    (:then
      (bind _actorspawned (Default|SpawnActor _asbp_top_down_controller (Variables|Default|GetActorClass) false))
      (Variables|/Game/Game/Blueprints/Spells/BP_Spells.BP_Spells_C|SetCurrentUser _actorspawned _asbp_top_down_controller)
      (Default|LaunchSpell _actorspawned)
      (return true))
    (:CastFailed
      (bind _asbp_enemy_ai_controller (Utilities|Casting|CastToBP_EnemyAI_Controller User))
      (bind _actorspawned_2 (Default|SpawnActor _asbp_enemy_ai_controller (Variables|Default|GetActorClass) false))
      (Variables|/Game/Game/Blueprints/Spells/BP_Spells.BP_Spells_C|SetCurrentUser _actorspawned_2 _asbp_enemy_ai_controller)
      (Default|LaunchSpell _actorspawned_2)
      (return true))))