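; BP_Interactable is an interactable actor with an empty Interact event and a prompt widget for the top-down character.
; Character overlap adds it to or removes it from the top-down controller's interactable list.
; On begin overlap the prompt shows if it is the controller's current, un-interacted target and hides if another is current; end overlap always hides it.
; Helper functions toggle the widget's visibility and set its WBP_InteractText text.
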(event Custom|Interact)

(event Collision|EventActorBeginOverlap
  (params (OtherActor :type Actor%20Object%20Reference))
  ;[0.15 0.15 0.15 0.5] Add interactable to array
  (Utilities|Casting|CastToBP_TopDownCharacter OtherActor)
  (Default|AddInteractable (CallFunction|GetTopDownController) self)
  (bind (_isvalid _currentinteractable) (Default|GetCurrentInteractable (CallFunction|GetTopDownController)))
  (if _isvalid
    (if (== _currentinteractable self)
      (if (not (Variables|BP_Interactable_C|GetIsInteracted _currentinteractable))
        (CallFunction|ShowInteractText))
      (else
        (CallFunction|HideInteractText)))))

(event Collision|EventActorEndOverlap
  (params (OtherActor :type Actor%20Object%20Reference))
  ;[0.15 0.15 0.15 0.5] Remove interactable from array and hide interact text
  (Utilities|Casting|CastToBP_TopDownCharacter OtherActor)
  (Default|RemoveInteractable (CallFunction|GetTopDownController) self)
  (CallFunction|HideInteractText))

(fn ConstructionScript)

(fn ShowInteractText
  (Rendering|SetVisibility (Variables|Default|GetInteractTextWidget) true false))

(fn HideInteractText
  (Rendering|SetVisibility (Variables|Default|GetInteractTextWidget) false false))

(fn SetInteractText
  (params (InteractText :type Text))
  (bind _aswbp_interact_text (Utilities|Casting|CastToWBP_InteractText (UserInterface|GetUserWidgetObject (Variables|Default|GetInteractTextWidget))))
  (Variables|/Script/UMG.TextBlock|SetText (Variables|/Game/Game/UI/Interactables/WBP_InteractText.WBP_InteractText_C|GetInteractText _aswbp_interact_text) InteractText))