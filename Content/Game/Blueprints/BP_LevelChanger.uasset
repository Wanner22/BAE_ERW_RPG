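; BP_LevelChanger is a trigger volume that moves the player to another level when the top-down character overlaps its box.
; On overlap it saves player info in the RPG game instance, fades out the camera, disables movement on the top-down controller and waits out the fade.
; It then stores a target player start tag in the game instance and opens the configured level.
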(event OnComponentBeginOverlap(Box)
  (params (OverlappedComponent :type Primitive%20Component%20Object%20Reference) (OtherActor :type Actor%20Object%20Reference) (OtherComp :type Primitive%20Component%20Object%20Reference) (OtherBodyIndex :type Integer) (bFromSweep :type Boolean) (SweepResult :type Hit%20Result%20Structure%20%28by%20ref%29))
  (bind _playercontroller (CallFunction|GetTopDownController))
  (Utilities|Casting|CastToBP_TopDownCharacter OtherActor)
  (Utilities|FlowControl|Sequence
    (:then_0
      (bind _asbp_gi_rpg (Utilities|Casting|CastToBP_GI_RPG (Game|GetGameInstance)))
      (Default|SavePlayerInfos _asbp_gi_rpg))
    (:then_1
      (bind _camerafadeduration (Default|CameraFadeOut _playercontroller))
      (Variables|/Game/TopDown/Blueprints/BP_TopDownController.BP_TopDownController_C|SetCanMove _playercontroller false)
      (Utilities|FlowControl|Delay _camerafadeduration)
      (CallFunction|GotoLevel))))

(fn ConstructionScript)

(fn GotoLevel
  (bind _asbp_gi_rpg (Utilities|Casting|CastToBP_GI_RPG (Game|GetGameInstance)))
  (Variables|/Game/Game/Blueprints/BP_GI_RPG.BP_GI_RPG_C|SetTargetPlayerStartTag _asbp_gi_rpg (Variables|Default|GetTargetPlayerStartTag))
  (Game|OpenLevel(byObjectReference) (Variables|Default|GetLevelToGo)))