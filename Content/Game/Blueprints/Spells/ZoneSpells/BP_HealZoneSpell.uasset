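; BP_HealZoneSpell is a zone spell that heals the player inside its sphere and destroys itself five seconds after spawning.
; A BP_TopDownCharacter beginning overlap triggers an immediate heal.
; Tick uses a one-second Delay as a throttle, healing again if player pawn 0 still overlaps the sphere afterwards.
; Both paths pass HealAmount to the top-down controller's Heal function.
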(event Custom|Heal
  (Default|Heal (CallFunction|GetTopDownController) (Variables|Default|GetHealAmount)))

(event EventBeginPlay
  (Utilities|FlowControl|Delay 5.0)
  (Actor|DestroyActor))

(event Collision|EventActorBeginOverlap
  (params (OtherActor :type Actor%20Object%20Reference))
  (Utilities|Casting|CastToBP_TopDownCharacter OtherActor)
  (CallFunction|Heal))

(event EventTick
  (params (DeltaSeconds :type Float%20%28single-precision%29))
  (if (Collision|IsOverlappingActor (Variables|Default|GetSphere) (Game|Player|GetPlayerPawn 0) :!class /Script/Engine.PrimitiveComponent)
    (Utilities|FlowControl|Delay 1.0)
    (if (Collision|IsOverlappingActor (Variables|Default|GetSphere) (Game|Player|GetPlayerPawn 0) :!class /Script/Engine.PrimitiveComponent)
      (CallFunction|Heal))))

(fn ConstructionScript)