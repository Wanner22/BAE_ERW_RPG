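; Interactable chest that opens once on interaction and adds its configured item to the top-down controller.
; On BeginPlay it sets the prompt text, loads the item's icon into a hidden widget and caches the icon's start and raised positions.
; Opening plays a lid-rotation timeline that hides the prompt, shows the icon and drives a second timeline lifting it.
; The icon hides again after a configurable delay.
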(event Custom|Open
  (if (not (Variables|Default|GetIsInteracted))
    (Variables|Default|SetIsInteracted true)
    ;[0.15 0.15 0.15 0.5] Open chest
    (bind _alpha (Timeline|LidRotation Play)
      (:Update
        (Transformation|SetRelativeRotation (Variables|Default|GetLid_Pivot) (Math|Rotator|Lerp(Rotator) "0, 0, 0" "120.000000,0.000000,0.000000" _alpha) false false)
        (Rendering|SetVisibility (Variables|Default|GetInteractTextWidget) false false)
        ;[0.15 0.15 0.15 0.5] Show object icon and moves it upwards
        (Rendering|SetVisibility (Variables|Default|GetObjectIcon) true false)
        (bind _alpha_2 (Timeline|ObjectIconLocation Play)
          (:Update
            (Transformation|SetRelativeLocation (Variables|Default|GetObjectIcon) (Math|Vector|Lerp(Vector) (Variables|Default|GetObjectIconCurrentLoc) (Variables|Default|GetObjectIconTargetLoc) _alpha_2) false false)
            (Utilities|FlowControl|Delay (Variables|Default|GetObjectVisDuration))
            (Rendering|SetVisibility (Variables|Default|GetObjectIcon) false false)))))))

(event EventBeginPlay
  (bind _objecticon (Variables|Default|GetObjectIcon))
  (bind _relativelocation (Variables|/Script/Engine.SceneComponent|GetRelativeLocation _objecticon))
  (CallFunction|SetInteractText "E to open")
  (bind _aswbp_object_icon (Utilities|Casting|CastToWBP_ObjectIcon (UserInterface|GetUserWidgetObject (Variables|Default|GetObjectIcon))))
  (Class|Image|SetBrush (Variables|/Game/Game/UI/Chest/WBP_ObjectIcon.WBP_ObjectIcon_C|GetObjectIcon _aswbp_object_icon) (Class|WidgetBlueprintLibrary|MakeBrushfromTexture (Variables|/Game/Game/Blueprints/Datas/BP_DA_Item.BP_DA_Item_C|GetIcon (Variables|Default|GetObject))))
  (Rendering|SetVisibility (Variables|Default|GetObjectIcon) false false)
  (Variables|Default|SetObjectIconCurrentLoc _relativelocation)
  (Variables|Default|SetObjectIconTargetLoc (+ _relativelocation "0.000000,0.000000,30.000000")))

(event Collision|EventActorBeginOverlap
  (params (OtherActor :type Actor%20Object%20Reference))
  (|CallParentFunction OtherActor) ; This node is disabled and will not be called.\nDrag off pins to build functionality.
)

(event EventTick
  (params (DeltaSeconds :type Float%20%28single-precision%29))
  (|CallParentFunction DeltaSeconds) ; This node is disabled and will not be called.\nDrag off pins to build functionality.
)

(event EventInteract
  (if (not (Variables|Default|GetIsInteracted))
    (CallFunction|Open)
    (Default|AddItem (CallFunction|GetTopDownController) (Variables|Default|GetObject))))

(fn ConstructionScript
  (|CallParentFunction))