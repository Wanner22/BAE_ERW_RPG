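; AI controller for enemies that runs the main behavior tree and stores the player pawn in its blackboard at BeginPlay.
; Attack uses a random entry from Spells, passing the controller as the caster.
; SpawnActor places actors ahead of the pawn, dropping zone spells to floor level using the capsule half-height.
; The controller also holds Hp, and TakeDamages destroys the pawn when it reaches zero.
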(event EventBeginPlay
  (bind _blackboardcomponent (Class|AIController|UseBlackboard "/Game/Game/AI/BB_MainBehaviourBlackBoard.BB_MainBehaviourBlackBoard"))
  (Variables|Default|SetBlackboard%20Component _blackboardcomponent)
  (AI|RunBehaviorTree "/Game/Game/AI/BT_MainBehaviour.BT_MainBehaviour")
  (AI|Components|Blackboard|SetValueasObject (Variables|Default|GetBlackboard%20Component) (Utilities|Name|MakeLiteralName "Player") (Game|Player|GetPlayerPawn 0)))

(event EventTick
  (params (DeltaSeconds :type Float%20%28single-precision%29)))

(fn ConstructionScript)

(fn Attack
  (Default|Use (.OutItem (Utilities|Array|Random (Variables|Default|GetSpells))) self))

(fn TakeDamages
  (params (HpToRemove :type Float%20%28double-precision%29))
  (CallFunction|UpdateHp (* HpToRemove -1.0))
  (if (<= (Variables|Default|GetHp) 0.0)
    (Actor|DestroyActor (Pawn|GetControlledPawn self))))

(fn UpdateHp
  (params (HpToAdd :type Float%20%28double-precision%29))
  (Variables|Default|SetHp (+ (Variables|Default|GetHp) HpToAdd)))

(fn SpawnActor
  (params (ActorToSpawn :type BP%20Spells%20Class%20Reference) (IsZoneSpell :type Boolean))
  (bind _returnvalue (Pawn|GetControlledPawn))
  (bind _returnvalue_2 (Pawn|GetControlledPawn))
  (bind _returnvalue_3 (Transformation|GetActorTransform _returnvalue))
  (bind _returnvalue_4 (Transformation|GetActorTransform _returnvalue_2))
  (if IsZoneSpell
    ;[0.15 0.15 0.15 0.5] If spell is a zone spell, spawn on floor
    (bind _asbp_top_down_enemy_character (Utilities|Casting|CastToBP_TopDownEnemy_Character (Pawn|GetControlledPawn)))
    (bind _returnvalue_5 (Game|SpawnActorfromClass ActorToSpawn (Math|Transform|MakeTransform (- (+ (.location _returnvalue_4) (* (Transformation|GetActorForwardVector _returnvalue_2) (Variables|Default|GetSpawnDistance))) (Math|Vector|MakeVector 0.0 0.0 (- (Variables|/Script/Engine.CapsuleComponent|GetCapsuleHalfHeight (Variables|/Script/Engine.Character|GetCapsuleComponent _asbp_top_down_enemy_character)) 1.0))) (.rotation _returnvalue_4) (.scale _returnvalue_4)) "Undefined" "MultiplyWithRoot" 0 0))
    (return _returnvalue_5)
    (else
      ;[0.15 0.15 0.15 0.5] If spell is not zone spell, spawn in front of enemy
      (bind _returnvalue_6 (Game|SpawnActorfromClass ActorToSpawn (Math|Transform|MakeTransform (+ (.location _returnvalue_3) (* (Transformation|GetActorForwardVector _returnvalue) (Variables|Default|GetSpawnDistance))) (.rotation _returnvalue_3) (.scale _returnvalue_3)) "Undefined" "MultiplyWithRoot" 0 0))
      (return _returnvalue_6))))