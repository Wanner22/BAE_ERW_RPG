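; Interactable Blueprint that steps through a list of dialogue lines on screen, with helpers for a camera close-up.
; Each Interact advances the text index and shows that line in the dialogue widget, then hides the widget and resets after the last.
; CameraToInteractable and CameraToPlayer blend the view, toggle the prompt and lock or restore top-down movement, but only a disconnected older toggle branch calls them here.
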(event Collision|EventActorBeginOverlap
  (params (OtherActor :type Actor%20Object%20Reference))
  (|CallParentFunction OtherActor) ; This node is disabled and will not be called.\nDrag off pins to build functionality.
)

(event EventBeginPlay
  (|CallParentFunction))

(event EventTick
  (params (DeltaSeconds :type Float%20%28single-precision%29))
  (|CallParentFunction DeltaSeconds) ; This node is disabled and will not be called.\nDrag off pins to build functionality.
)

(event EventInteract
  (Math|Integer|IncrementInt (Variables|Default|GetTextIndex)
    (:%20%20
      (if (< (Variables|Default|GetTextIndex) (Utilities|Array|Length (Variables|Default|GetDialogueTexts)))
        (Variables|/Script/UMG.TextBlock|SetText (Variables|/Game/Game/Blueprints/UI/WBP_Dialogue.WBP_Dialogue_C|GetDialogueText (Variables|Default|GetDialogueWidget)) (Utilities|Array|Get(acopy) (Variables|Default|GetDialogueTexts) (Variables|Default|GetTextIndex)))
        (CallFunction|ShowDialogueWidget)
        (else
          (Variables|Default|SetTextIndex -1)
          (CallFunction|HideDialogueWidget))))))

(fn ConstructionScript
  (|CallParentFunction))

(fn CameratoInteractable
  (bind _playercontroller (CallFunction|GetTopDownController))
  ;[0.15 0.15 0.15 0.5] Camera to interactabale
  (Game|Player|SetViewTargetwithBlend _playercontroller self 0.7 "VTBlend_Linear" 0.0 false)
  (Rendering|SetVisibility (Variables|Default|GetInteractText) false false)
  (Variables|/Game/TopDown/Blueprints/BP_TopDownController.BP_TopDownController_C|SetCanMove _playercontroller false))

(fn CameratoPlayer
  (bind _playercontroller (CallFunction|GetTopDownController))
  ;[0.15 0.15 0.15 0.5] Camera to player
  (Game|Player|SetViewTargetwithBlend _playercontroller (Pawn|GetControlledPawn _playercontroller) 0.7 "VTBlend_Linear" 0.0 false)
  (Rendering|SetVisibility (Variables|Default|GetInteractText) true false)
  (Variables|/Game/TopDown/Blueprints/BP_TopDownController.BP_TopDownController_C|SetCanMove _playercontroller true))

(fn ShowDialogueWidget
  (bind _dialoguewidget (Variables|Default|GetDialogueWidget))
  (if (not (Widget|IsVisible _dialoguewidget))
    (UserInterface|Viewport|AddtoViewport _dialoguewidget 0)))

(fn HideDialogueWidget
  (bind _dialoguewidget (Variables|Default|GetDialogueWidget))
  (if (Widget|IsVisible _dialoguewidget)
    (Widget|RemovefromParent _dialoguewidget)))